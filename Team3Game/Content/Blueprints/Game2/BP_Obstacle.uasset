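; BP_Obstacle is an obstacle actor that ends the game when a player pawn hits it.
; On mesh overlap with a BP_PawnBase, it calls HitObstacle on the pawn, then GameOver on the level manager, printing a warning if none is found.
; The construction script randomizes the mesh's vertical scale for height variety.
; Getter and setter functions store a parent reference, which the obstacle itself does not otherwise use.
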(event `self.StaticMesh.OnComponentBeginOverlap`
  (params (OverlappedComponent :type "PrimitiveComponent Object Reference") (OtherActor :type "Actor Object Reference") (OtherComp :type "PrimitiveComponent Object Reference") (OtherBodyIndex :type Integer) (bFromSweep :type Boolean) (SweepResult :type "HitResult Structure (by ref)"))
  (bind (_levelmanager _levelmanagerfound) (`/Game/Blueprints/Game2/BPF_Lib.GetLevelManager`))
  (bind _asbp_pawn_base (cast `/Game/Blueprints/Game2/BP_PawnBase` OtherActor))
  (`/Game/Blueprints/Game2/BP_PawnBase.HitObstacle` _asbp_pawn_base)
  (if _levelmanagerfound
    (`/Game/Blueprints/Game2/BP_LevelManager.GameOver` _levelmanager)
    (else
      (`KismetSystemLibrary.PrintString` "Level Manager Not Found"))))

(fn `ReturnParent`
  (returns (Parent :type "/Game/Blueprints/Game2/BP_SpawnerBase Object Reference"))
  (return (`self.ParentRef`)))

(fn `SetParent`
  (params (SetParent :type "/Game/Blueprints/Game2/BP_SpawnerBase Object Reference"))
  (returns (Return :type Boolean))
  (set `self.ParentRef` SetParent)
  (return false))

(fn `UserConstructionScript`
  (`SceneComponent.SetWorldScale3D` (`self.StaticMesh`) (`KismetMathLibrary.MakeVector` 1.0 1.0 (`KismetMathLibrary.RandomFloatInRange` 1.0 3.0))))