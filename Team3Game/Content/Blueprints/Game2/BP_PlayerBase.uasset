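; BP_PlayerBase is the player pawn for a lane-based dodging game, reading lane count, width and play state from a level manager.
; A and D slide it one lane sideways via timelines, guarded against edges and overlapping moves.
; Game start animates its dynamic material colour, then turns on exhaust particles.
; Hitting an obstacle spawns an explosion, hides the player and blends to a tagged end camera.
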(event `Key|A`
  (params (Key :type "Key Structure"))
  (bind (_returnvalue_x _returnvalue_y) (`KismetMathLibrary.BreakVector` (`self.K2_GetActorLocation`)))
  (bind (_returnvalue_x_2 _returnvalue_y_2 _returnvalue_z) (`KismetMathLibrary.BreakVector` (`self.K2_GetActorLocation`)))
  (:`Pressed`
    (if (`/Game/Blueprints/Game2/BP_LevelManager.bPlaying` (`self.LevelManagerRef`))
      ;[1 1 1] Pressed Left in the Left most lane
      (if (<= (`self.CurrentLane`) 1)
        _
        (elif (not (`self.bMoving`))
          (set `self.bMoving` true)
          (set `self.TargetPosition` (- _returnvalue_y (`self.LaneWidth`)))
          (bind (_direction _move) (`Timeline|MoveLeft` :!via `PlayFromStart`)
            (:`Update`
              (`self.K2_SetActorLocation` (`KismetMathLibrary.MakeVector` _returnvalue_x_2 (`KismetMathLibrary.Lerp` _returnvalue_y_2 (`self.TargetPosition`) _move) _returnvalue_z)))
            (:`Finished`
              (set `self.bMoving` false)
              (`/Engine/EditorBlueprintResources/StandardMacros.DecrementInt` (`self.CurrentLane`)))))))))

(event `Key|D`
  (params (Key :type "Key Structure"))
  (bind (_returnvalue_x _returnvalue_y) (`KismetMathLibrary.BreakVector` (`self.K2_GetActorLocation`)))
  (bind (_returnvalue_x_2 _returnvalue_y_2 _returnvalue_z) (`KismetMathLibrary.BreakVector` (`self.K2_GetActorLocation`)))
  (:`Pressed`
    (if (`/Game/Blueprints/Game2/BP_LevelManager.bPlaying` (`self.LevelManagerRef`))
      ;[1 1 1] Pressed Right when in right most lane
      (if (== (`self.CurrentLane`) (`/Game/Blueprints/Game2/BP_LevelManager.NumberOfLanes` (`self.LevelManagerRef`)))
        _
        (elif (not (`self.bMoving`))
          (set `self.bMoving` true)
          (set `self.TargetPosition` (+ _returnvalue_y (`self.LaneWidth`)))
          (bind (_direction _move) (`Timeline|MoveRight` :!via `PlayFromStart`)
            (:`Update`
              (`self.K2_SetActorLocation` (`KismetMathLibrary.MakeVector` _returnvalue_x_2 (`KismetMathLibrary.Lerp` _returnvalue_y_2 (`self.TargetPosition`) _move) _returnvalue_z)))
            (:`Finished`
              (set `self.bMoving` false)
              (`/Engine/EditorBlueprintResources/StandardMacros.IncrementInt` (`self.CurrentLane`)))))))))

(event `GameStarted`
  ;[1 1 1] Lerp Player colour and then start thruster emitter
  (bind (_direction _colourchange) (`Timeline|AnimateColour` :!via `PlayFromStart`)
    (:`Update`
      (`MaterialInstanceDynamic.SetVectorParameterValue` (`self.PlayerMaterial`) "Colour" (`KismetMathLibrary.LinearColorLerp` (`self.PlayerStartColour`) (`self.PlayerEndColour`) _colourchange)))
    (:`Finished`
      (`ParticleSystemComponent.SetTemplate` (`self.ParticleSystem`) "/Game/Assets/Effects/P_Exhaust.P_Exhaust"))))

(fn `HitObstacle`
  (`ActorComponent.K2_DestroyComponent` (`self.ParticleSystem`))
  (`GameplayStatics.SpawnEmitterAtLocation` "/Game/Assets/Effects/P_Explode.P_Explode" (`self.K2_GetActorLocation`))
  (`PlayerController.SetViewTargetWithBlend` (`GameplayStatics.GetPlayerController` 0) (`self.EndCam`) 1.0 "VTBlend_Linear" 0.0 false)
  (`SceneComponent.ToggleVisibility` (`self.Player`) false))

(fn `Initialise`
  (bind (_levelmanager _levelmanagerfound) (`/Game/Blueprints/Game2/BP_Lib.GetLevelManager`))
  (if _levelmanagerfound
    (set `self.LevelManagerRef` _levelmanager)
    (set `self.CurrentLane` (+ (/ (`/Game/Blueprints/Game2/BP_LevelManager.NumberOfLanes` (`self.LevelManagerRef`)) 2) 1))
    (set `self.LaneWidth` (`/Game/Blueprints/Game2/BP_LevelManager.LaneWidth` (`self.LevelManagerRef`)))
    ;[1 1 1] Create dynamic material for player colour change
    (bind _returnvalue (`PrimitiveComponent.CreateDynamicMaterialInstance` (`self.Player`) 0 null "None"))
    (bind _output_get (set `self.PlayerMaterial` _returnvalue))
    (`MaterialInstanceDynamic.SetVectorParameterValue` _output_get "Colour" (`self.PlayerStartColour`))
    (bind _outactors (`GameplayStatics.GetAllActorsWithTag` "EndCam"))
    (set `self.EndCam` (`|GetArrayItem` _outactors))
    (else
      (`KismetSystemLibrary.PrintString` "No Level Manager Found"))))

(fn `UserConstructionScript`
  (`self.Initialise`))