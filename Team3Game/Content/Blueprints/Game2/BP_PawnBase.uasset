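; Base player pawn for a lane-based game, stepping sideways between lanes on A and D while the level manager reports play.
; On BeginPlay it reads lane count and width from the level manager, sets a middle starting lane and caches an EndCam-tagged actor.
; Timelines lerp current Y toward the next lane, with a Moving flag blocking overlapping moves and edge checks limiting range.
; HitObstacle hides the Player component.
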(event `self.ReceiveBeginPlay`
  (`self.Intialize `))

(event `Key|A`
  (params (Key :type "Key Structure"))
  (bind (_returnvalue_x _returnvalue_y) (`KismetMathLibrary.BreakVector` (`self.K2_GetActorLocation`)))
  (bind (_returnvalue_x_2 _returnvalue_y_2 _returnvalue_z) (`KismetMathLibrary.BreakVector` (`self.K2_GetActorLocation`)))
  (:`Pressed`
    (if (`/Game/Blueprints/Game2/BP_LevelManager.bIsPlaying` (`self.LevelManagerRef`))
      ;[1 1 1] Pressed Left whilst in left most lane
      (if (<= (`self.CurrentLane`) 1)
        _
        (elif (not (`self.bMoving`))
          (set `self.bMoving` true)
          (set `self.TargetPosition` (- _returnvalue_y (`self.LaneWidth`)))
          (bind (_direction _move) (`Timeline|MoveLeft` :!via `PlayFromStart`)
            (:`Update`
              (`self.K2_SetActorLocation` (`KismetMathLibrary.MakeVector` _returnvalue_x_2 (`KismetMathLibrary.Lerp` _returnvalue_y_2 (`self.TargetPosition`) _move) _returnvalue_z)))
            (:`Finished`
              (set `self.bMoving` false)
              (`/Engine/EditorBlueprintResources/StandardMacros.DecrementInt` (`self.CurrentLane`)))))))))

(event `Key|D`
  (params (Key :type "Key Structure"))
  (bind (_returnvalue_x _returnvalue_y) (`KismetMathLibrary.BreakVector` (`self.K2_GetActorLocation`)))
  (bind (_returnvalue_x_2 _returnvalue_y_2 _returnvalue_z) (`KismetMathLibrary.BreakVector` (`self.K2_GetActorLocation`)))
  (:`Pressed`
    (if (`/Game/Blueprints/Game2/BP_LevelManager.bIsPlaying` (`self.LevelManagerRef`))
      ;[1 1 1] Check if we pressed right in the right most lane
      (if (== (`self.CurrentLane`) (`/Game/Blueprints/Game2/BP_LevelManager.NumberOfLanes` (`self.LevelManagerRef`)))
        _
        (elif (not (`self.bMoving`))
          (set `self.bMoving` true)
          (set `self.TargetPosition` (+ _returnvalue_y (`self.LaneWidth`)))
          (bind (_direction _move) (`Timeline|MoveRight` :!via `PlayFromStart`)
            (:`Update`
              (`self.K2_SetActorLocation` (`KismetMathLibrary.MakeVector` _returnvalue_x_2 (`KismetMathLibrary.Lerp` _returnvalue_y_2 (`self.TargetPosition`) _move) _returnvalue_z)))
            (:`Finished`
              (set `self.bMoving` false)
              (`/Engine/EditorBlueprintResources/StandardMacros.IncrementInt` (`self.CurrentLane`)))))))))

(fn `HitObstacle`
  (`SceneComponent.ToggleVisibility` (`self.Player`) false))

(fn `Intialize `
  (bind (_levelmanager _levelmanagerfound) (`/Game/Blueprints/Game2/BPF_Lib.GetLevelManager`))
  (if _levelmanagerfound
    (set `self.LevelManagerRef` _levelmanager)
    (set `self.CurrentLane` (+ (/ (`/Game/Blueprints/Game2/BP_LevelManager.NumberOfLanes` (`self.LevelManagerRef`)) 2) 1))
    (set `self.LaneWidth` (`/Game/Blueprints/Game2/BP_LevelManager.LaneWidth` (`self.LevelManagerRef`)))
    (bind _outactors (`GameplayStatics.GetAllActorsWithTag` "EndCam"))
    (set `self.EndCam` (`|GetArrayItem` _outactors))
    (else
      (`KismetSystemLibrary.PrintString` "Level Manager Missing"))))

(fn `UserConstructionScript`)