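; Obstacle spawner, derived from a parent spawner, that places obstacles at random intervals while the level manager reports play is active.
; BeginPlay starts a self-repeating delay loop and immediately places one obstacle, whose X is randomized if SpawnVisualObstacle is set.
; Each loop pass spawns an obstacle through the parent's SpawnActor at the spawner's location, then checks Playing before repeating.
; Obstacles reported as hitting bounds are destroyed.
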(event `self.ReceiveBeginPlay`
  (`parent.ReceiveBeginPlay`)
  (set `self.LevelManagerRef` (`/Game/Blueprints/Game2/BP_Lib.GetLevelManager`))
  (`self.LineUpNextObstacleSpawn`)
  (`self.PlaceObstacle` (`self.bSpawnVisualObstacle`)))

(event `LineUpNextObstacleSpawn`
  (`KismetSystemLibrary.Delay` (`KismetMathLibrary.RandomFloatInRange` (`self.MinDelay`) (`self.MaxDelay`)))
  (`self.PlaceObstacle` false)
  (if (`/Game/Blueprints/Game2/BP_LevelManager.bPlaying` (`self.LevelManagerRef`))
    (`self.LineUpNextObstacleSpawn`)))

(event `self.SpawnedActorHitBounds`
  (params (OutOfBoundsActor :type "Actor Object Reference"))
  ;[1 1 1] Destroy Spawned Obstacle
  (`self.K2_DestroyActor` OutOfBoundsActor))

(fn `PlaceObstacle`
  (params (OverrideLocation :type Boolean))
  (bind (_returnvalue_x _returnvalue_y _returnvalue_z) (`KismetMathLibrary.BreakVector` (`self.K2_GetActorLocation`)))
  (bind _spawnedactor (`self.SpawnActor`))
  (`self.K2_SetActorLocation` _spawnedactor (select `bool` OverrideLocation :`false` (`self.K2_GetActorLocation`) :`true` (`KismetMathLibrary.MakeVector` (`KismetMathLibrary.RandomFloatInRange` -100.0 100.0) _returnvalue_y _returnvalue_z)) false false))

(fn `SpawnActor`
  (returns (SpawnedActor :type "Actor Object Reference"))
  (bind _spawnedactor (`parent.SpawnActor`))
  (return _spawnedactor))

(fn `UserConstructionScript`
  (`parent.UserConstructionScript`))