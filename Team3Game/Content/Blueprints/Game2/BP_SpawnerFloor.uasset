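; BP_SpawnerFloor is a child spawner that builds a looping floor from a fixed pool of tiles.
; BeginPlay spawns the tiles through the parent's SpawnActor, measures tile width from the first one's bounds, and lines up the rest along X.
; SpawnedActorHitBounds recycles an out-of-bounds tile by moving it behind the tracked RearTile, making it the new rear.
; A "First" tag on the initial tile applies a small offset workaround when repositioning.
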(event `self.ReceiveBeginPlay`
  (bind (_returnvalue_x _returnvalue_y) (`KismetMathLibrary.BreakVector` (`self.K2_GetActorLocation`)))
  (bind (_returnvalue_x_2 _returnvalue_y_2) (`KismetMathLibrary.BreakVector` (`self.K2_GetActorLocation` (`self.RearTile`))))
  (`parent.ReceiveBeginPlay`)
  (for _index (range (`self.ActorsRequired`))
    (if (== _index 0)
      (bind _spawnedactor (`self.SpawnActor`))
      (set `self.RearTile` _spawnedactor)
      (bind _output_get (set `self.TileSize` (* (.x (`.BoxExtent` (`self.GetActorBounds` _spawnedactor false false))) 2.0)))
      (`self.K2_SetActorLocation` (`KismetMathLibrary.MakeVector` _output_get _returnvalue_y))
      ;[1 1 1] Fix for weird behaviour
      (set `Actor.Tags` (`|MakeArray` "First" :!type "Name") (`self.RearTile`))
      (else
        (bind _spawnedactor_2 (`self.SpawnActor`))
        (`self.K2_SetActorLocation` _spawnedactor_2 (`KismetMathLibrary.MakeVector` (+ _returnvalue_x_2 (`self.TileSize`)) _returnvalue_y_2) false false)
        (bind _output_get_2 (set `self.RearTile` _spawnedactor_2))
        (message `/Game/Blueprints/Game2/BPI_Spawnable.SetParent` _output_get_2 self)))))

(event `self.SpawnedActorHitBounds`
  (params (OutOfBoundsActor :type "Actor Object Reference"))
  (bind (_returnvalue_x _returnvalue_y) (`KismetMathLibrary.BreakVector` (`self.K2_GetActorLocation` (`self.RearTile`))))
  ;[1 1 1] Move Floor to new location
  (`self.K2_SetActorLocation` OutOfBoundsActor (`KismetMathLibrary.MakeVector` (+ _returnvalue_x (- (`self.TileSize`) (`KismetMathLibrary.SelectFloat` 5.0 0.0 (`self.ActorHasTag` OutOfBoundsActor "First")))) _returnvalue_y) false false)
  (set `self.RearTile` OutOfBoundsActor))

(fn `SpawnActor`
  (returns (SpawnedActor :type "Actor Object Reference"))
  (bind _spawnedactor (`parent.SpawnActor`))
  (return _spawnedactor))

(fn `UserConstructionScript`
  (`parent.UserConstructionScript`))