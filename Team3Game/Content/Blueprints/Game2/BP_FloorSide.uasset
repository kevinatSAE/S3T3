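; BP_FloorSide is a scatter Blueprint that fills a box volume with randomly sized mesh instances, apparently as dressing along the side of a floor.
; Its construction script moves the InstancedStaticMesh to the Box's relative location, applied as a world location, then clears and rebuilds a small fixed number of instances.
; Each instance gets a random point within the Box bounds, random X and Y scales between MinXY and MaxXY, and a separately randomized height scale.
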(fn `UserConstructionScript`
  (bind _instancedstaticmesh (`self.InstancedStaticMesh`))
  (bind _minxy (`self.MinXY`))
  (bind _maxxy (`self.MaxXY`))
  (bind (_origin _boxextent) (`KismetSystemLibrary.GetComponentBounds` (`self.Box`)))
  (`parent.UserConstructionScript`)
  (`SceneComponent.K2_SetWorldLocation` _instancedstaticmesh (`SceneComponent.RelativeLocation` (`self.Box`)) false false)
  (`InstancedStaticMeshComponent.ClearInstances` _instancedstaticmesh)
  (for _ (range 11)
    (`InstancedStaticMeshComponent.AddInstance` _instancedstaticmesh (`KismetMathLibrary.MakeTransform` (`KismetMathLibrary.RandomPointInBoundingBox` _origin _boxextent) (struct) (`KismetMathLibrary.MakeVector` (`KismetMathLibrary.RandomFloatInRange` _minxy _maxxy) (`KismetMathLibrary.RandomFloatInRange` _minxy _maxxy) (`KismetMathLibrary.RandomFloatInRange` 5.0 20.0))))))