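; BoulderSpawner is an actor that repeatedly spawns Boulder actors at the world position of its Sphere component.
; Tick drives a Delay node as a repeating timer, waiting Timer plus StartDelay before each spawn.
; StartDelay is zeroed after spawning, so it only offsets the first boulder.
; Each boulder gets a random rotation, including roll, and the scale set by BoulderScale.
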(event `self.ReceiveTick`
  (params (DeltaSeconds :type "Float (single-precision)"))
  (`KismetSystemLibrary.Delay` (+ (`self.Timer`) (`self.StartDelay`)))
  (`|SpawnActorFromClass` "/Game/Blueprints/Game1/Boulder.Boulder_C" (`KismetMathLibrary.MakeTransform` (`KismetMathLibrary.TransformLocation` (`SceneComponent.K2_GetComponentToWorld` (`self.Sphere`))) (`KismetMathLibrary.RandomRotator` true) (`self.BoulderScale`)) "Undefined" "OverrideRootScale" null null)
  (set `self.StartDelay` 0.0))

(fn `UserConstructionScript`)